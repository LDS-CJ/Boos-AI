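; Blueprint function library of helpers for the Boss character, covering chance rolls and movement speed.
; Maybe treats its input as a percentage clamped to 0–100 and returns true when it beats a random float in that range.
; SetSpeed casts the target to Boss and sets its max walk speed from a Walk, Run or Free selector, using fixed presets or, for Free, the supplied speed.
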(fn `Maybe`
  (params (Num :type "Float (double-precision)"))
  (returns (Return :type Boolean))
  (return (> (`KismetMathLibrary.FClamp` Num 0.0 100.0) (`KismetMathLibrary.RandomFloatInRange` 0.0 100.0))))

(fn `Set Speed`
  (params (Target :type "Character Object Reference") (index :type "/Game/Boss/Enum/SpeedType Enum" :default "NewEnumerator0") (Speed :type "Float (double-precision)"))
  (bind (_walk _run) (break `/Game/Boss/BluePrints/Structs/Boos_Speed` (make `/Game/Boss/BluePrints/Structs/Boos_Speed` 300.0)))
  (bind _asboss (cast `/Game/Boss/BluePrints/Boss` Target))
  (set `CharacterMovementComponent.MaxWalkSpeed` (select `/Game/Boss/Enum/SpeedType` index :`NewEnumerator0` _walk :`NewEnumerator1` _run :`NewEnumerator2` Speed) (`Character.CharacterMovement` _asboss)))