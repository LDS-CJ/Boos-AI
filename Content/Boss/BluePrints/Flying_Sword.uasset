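; Flying sword projectile Blueprint for a boss, built around a ProjectileMovement component.
; The construction script sets its initial speed and randomizes the maximum speed per instance.
; BeginPlay stores the spawn location for a release timeline that would raise the sword vertically, then activate projectile movement when finished.
; Nothing in this file starts that timeline, so the rise-and-launch sequence never runs.
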(event `self.ReceiveBeginPlay`
  (set `self.ActorLocation` (`self.K2_GetActorLocation`)))

(fn `UserConstructionScript`
  (bind _projectilemovement (`self.ProjectileMovement`))
  (set `ProjectileMovementComponent.InitialSpeed` 2000.0 _projectilemovement)
  (set `ProjectileMovementComponent.MaxSpeed` (`KismetMathLibrary.RandomFloatInRange` 2500.0 3000.0) _projectilemovement))