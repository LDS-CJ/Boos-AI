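; Boss actor Blueprint that provides movement and weapon-trace events for a boss.
; Dodge steps the boss backward and BaseMove moves it by a given step after a delay, both using timeline curves to lerp a swept location.
; BaseMove re-reads the forward vector on each update, while Dodge captures it once.
; AttractTrace box-traces between the weapon's Begin and End sockets with persistent debug drawing, leaving hits unused.
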(event `Dodge`
  (bind _current_location (`self.Current Location`))
  (set `self.Current Location` (`self.K2_GetActorLocation`))
  (set `self.Forward Vector` (`self.GetActorForwardVector`))
  (bind (_direction `_后撤步曲线`) (`Timeline|后撤步` :!via `PlayFromStart`)
    (:`Update`
      (`self.K2_SetActorLocation` (`KismetMathLibrary.VLerp` _current_location (+ _current_location (* (`self.Forward Vector`) -500)) `_后撤步曲线`) true))))

(event `BaseMove`
  (params (Step :type Integer) (Duration :type "Float (double-precision)"))
  (bind _current_location (`self.Current Location`))
  (`KismetSystemLibrary.Delay` Duration)
  (set `self.Current Location` (`self.K2_GetActorLocation`))
  (bind (_direction `_后撤步曲线`) (`Timeline|时间轴_0` :!via `PlayFromStart`)
    (:`Update`
      (`self.K2_SetActorLocation` (`KismetMathLibrary.VLerp` _current_location (+ _current_location (* (`self.GetActorForwardVector`) Step)) `_后撤步曲线`) true))))

(event `AttractTrace`
  (bind _weapon (`self.Weapon`))
  (`KismetSystemLibrary.BoxTraceSingle` :`Start` (`SceneComponent.GetSocketLocation` _weapon "Begin") :`End` (`SceneComponent.GetSocketLocation` _weapon "End") :`HalfSize` (1.0 1.0 1.0) :`TraceChannel` "TraceTypeQuery1" :`DrawDebugType` "Persistent"))

(fn `UserConstructionScript`)